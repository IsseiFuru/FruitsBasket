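; Game mode for the fruit-separating game that sets up and times a single round.
; On BeginPlay it resets the game instance's cursor list, tuning values and score, adds the main HUD, and spawns the OSC receiver and fruit spawner actors.
; A looping one-second timer decrements the game instance's countdown and, at zero, opens the End level after a short delay.
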(event `self.ReceiveBeginPlay`
  (`self.InitialGameInstance`)
  (`self.Create UI`)
  (`self.Timer`)
  (`self.SpawnOscReceiver`)
  (`self.SpawnFruitsSpawner`))

(event `InitialGameInstance`
  (bind _asseparate_fruits_game_instance (`/Game/BP/BPL_Utility.GetGameInstanceRef`))
  (bind _output_get (set `self.As Separate Fruits Game Instance` _asseparate_fruits_game_instance))
  (set `/Game/BP/SeparateFruitsGameInstance.CursorList` (`/Game/BP/SeparateFruitsGameInstance.DefaultCursorList` _output_get) _output_get)
  (set `/Game/BP/SeparateFruitsGameInstance.MinimumDistance` 0.2 _output_get)
  (set `/Game/BP/SeparateFruitsGameInstance.MaxFruits` 1 _output_get)
  (set `/Game/BP/SeparateFruitsGameInstance.Second` 60 _output_get)
  (set `/Game/BP/SeparateFruitsGameInstance.Score` 0 _output_get))

(event `Create UI`
  (bind _returnvalue (`|CreateWidget` "/Game/UI/WBP_Main.WBP_Main_C"))
  (`UserWidget.AddToViewport` _returnvalue 0))

(event `Timer`
  (`KismetSystemLibrary.K2_SetTimerDelegate` (delegate `CountDown`) 1.0 true))

(event `CountDown`
  (bind _as_separate_fruits_game_instance (`self.As Separate Fruits Game Instance`))
  (bind _second (`/Game/BP/SeparateFruitsGameInstance.Second` _as_separate_fruits_game_instance))
  (if (not (== _second 0))
    (bind _output_get (set `/Game/BP/SeparateFruitsGameInstance.Second` (- _second 1) _as_separate_fruits_game_instance))
    (if (== _output_get 0)
      (`KismetSystemLibrary.Delay` 2.0)
      (`GameplayStatics.OpenLevelBySoftObjectPtr` "/Game/Map/End.End"))))

(event `SpawnOscReceiver`
  (`|SpawnActorFromClass` "/Game/BP/BP_OscReceiver.BP_OscReceiver_C" (`self.NoneStaticMeshTransform`) "Undefined" "OverrideRootScale" null null))

(event `SpawnFruitsSpawner`
  (`|SpawnActorFromClass` "/Game/BP/BP_FruitsSpawner.BP_FruitsSpawner_C" (`self.NoneStaticMeshTransform`) "Undefined" "OverrideRootScale" null null))

(fn `UserConstructionScript`)