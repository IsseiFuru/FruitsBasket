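; BP_OscReceiver is an actor that receives cursor input over OSC and shares it through the game instance.
; On BeginPlay it starts an OSC server, and each received bundle's messages are parsed into cursor structs with state, session ID and position.
; Cursors with session IDs up to 1 overwrite their CursorList slot, identically for add, update and remove.
; Tick destroys the actor when the game instance's Second reaches zero.
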(event `self.ReceiveBeginPlay`
  (bind _returnvalue (`OSCManager.CreateOSCServer` "0.0.0.0" 50000 false true "" self))
  (add `OSCServer.OnOscBundleReceived` _returnvalue (delegate `OscMessageAnalysis`)))

(event `OscMessageAnalysis`
  (params (Bundle :type "OSCBundle Structure (by ref)") (IPAddress :type String) (Port :type Integer))
  (bind (_currentcursor_state _currentcursor_sessionid _currentcursor_psition) (break `/Game/BP/F_Cursor` (`self.CurrentCursor`)))
  (bind (_currentcursor_state_2 _currentcursor_sessionid_2 _currentcursor_psition_2) (break `/Game/BP/F_Cursor` (`self.CurrentCursor`)))
  (bind (_currentcursor_state_3 _currentcursor_sessionid_3 _currentcursor_psition_3) (break `/Game/BP/F_Cursor` (`self.CurrentCursor`)))
  (bind _returnvalue (`OSCManager.GetMessagesFromBundle` Bundle))
  (for _array_element _returnvalue
    (bind _f_cursol (`self.FillterOscAnalysis` _array_element))
    (bind _output_get (set `self.CurrentCursor` _f_cursol))
    (if (<= (`.SessionID_9_A8C2F19D4D3689F4225F5B8861A03225` (break `/Game/BP/F_Cursor` _output_get)) 1)
      (bind _asseparate_fruits_game_instance (`/Game/BP/BPL_Utility.GetGameInstanceRef`))
      (switch `string` (break `/Game/BP/F_Cursor` _output_get)
        (:`add`
          (bind _cursorlist (`/Game/BP/SeparateFruitsGameInstance.CursorList` _asseparate_fruits_game_instance))
          ;[1 1 1] add
          (`KismetArrayLibrary.Array_Set` _cursorlist _currentcursor_sessionid_2 (make `/Game/BP/F_Cursor` _currentcursor_state_2 _currentcursor_sessionid_2 _currentcursor_psition_2)))
        (:`update`
          ;[1 1 1] update
          (`KismetArrayLibrary.Array_Set` _cursorlist _currentcursor_sessionid_3 (make `/Game/BP/F_Cursor` _currentcursor_state_3 _currentcursor_sessionid_3 _currentcursor_psition_3)))
        (:`remove`
          ;[1 1 1] remove
          (`KismetArrayLibrary.Array_Set` _cursorlist _currentcursor_sessionid (make `/Game/BP/F_Cursor` _currentcursor_state _currentcursor_sessionid _currentcursor_psition)))))))

(event `self.ReceiveTick`
  (params (DeltaSeconds :type "Float (single-precision)"))
  (bind _asseparate_fruits_game_instance (`/Game/BP/BPL_Utility.GetGameInstanceRef`))
  (if (== (`/Game/BP/SeparateFruitsGameInstance.Second` _asseparate_fruits_game_instance) 0)
    (`self.K2_DestroyActor` self)))

(fn `FillterOscAnalysis`
  (params (OscMessage :type "OSCMessage Structure (by ref)"))
  (returns (F_Cursol :type "/Game/BP/F_Cursor Structure"))
  (locals (Y :type "Float (single-precision)") (X :type "Float (single-precision)") (SessionID :type Integer) (State :type String))
  (bind _state (`local.State`))
  (`|ExecutionSequence`
    (:`then_0`
      (bind _value (`OSCManager.GetString` OscMessage))
      (set `local.State` _value)
      (bind _value_2 (`OSCManager.GetInt32` OscMessage 1))
      (set `local.SessionID` _value_2))
    (:`then_1`
      (if (or (`KismetStringLibrary.EqualEqual_StrStr` _state "add") (`KismetStringLibrary.EqualEqual_StrStr` _state "update"))
        (bind _value_3 (`OSCManager.GetFloat` OscMessage 2))
        (set `local.X` _value_3)
        (bind _value_4 (`OSCManager.GetFloat` OscMessage 3))
        (set `local.Y` _value_4)))
    (:`then_2`
      (return (make `/Game/BP/F_Cursor` (`local.State`) (`local.SessionID`) (`KismetMathLibrary.MakeVector2D` (`local.X`) (`local.Y`)))))))

(fn `UserConstructionScript`)