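; Pear fruit actor that scores when it lands in a matching pear basket and removes itself after contact.
; On overlap, it casts the other actor to BP_PearBasket and adds points to the game instance's Score if their FruitsNumber values match.
; After a short delay following any overlap, it destroys itself and decrements the game instance's FruitsCount.
; The construction script enables CCD on the static mesh.
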(event `self.ReceiveActorBeginOverlap`
  (params (OtherActor :type "Actor Object Reference"))
  (bind _asseparate_fruits_game_instance (`/Game/BP/BPL_Utility.GetGameInstanceRef`))
  (bind _asbp_pear_basket (cast `/Game/BP/BP_PearBasket` OtherActor)
    (:`then`
      (if (== (`/Game/BP/BP_PearBasket.FruitsNumber` _asbp_pear_basket) (`self.FruitsNumber`))
        (set `/Game/BP/SeparateFruitsGameInstance.Score` (+ (`/Game/BP/SeparateFruitsGameInstance.Score` _asseparate_fruits_game_instance) 1000) _asseparate_fruits_game_instance)))
    (:`CastFailed`
      _))
  (`KismetSystemLibrary.Delay` 0.3)
  (`self.K2_DestroyActor`)
  (set `/Game/BP/SeparateFruitsGameInstance.FruitsCount` (- (`/Game/BP/SeparateFruitsGameInstance.FruitsCount` _asseparate_fruits_game_instance) 1) _asseparate_fruits_game_instance))

(fn `UserConstructionScript`
  (`PrimitiveComponent.SetUseCCD` (`self.StaticMesh`) true "None"))