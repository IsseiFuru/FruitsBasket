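; BP_Bar is a bar actor in a fruit-separating game (SeparateFruits), driven by two tracked cursors.
; Each Tick counts GameInstance cursors in Add or Update state; with exactly two, far enough apart, it applies GetBarTransform's position, rotation and scale, converting measured position to world.
; Otherwise it destroys itself after a short delay.
; The construction script enables CCD on the Bar component.
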(event `self.ReceiveTick`
  (params (DeltaSeconds :type "Float (single-precision)"))
  (set `self.CousorCount` 0)
  (bind _asfruits_basket_game_instance (`/Game/BP/BPL_Utility.GetGameInstanceRef`))
  (bind _output_get (set `self.As Separate Fruits Game Instance` _asfruits_basket_game_instance))
  (if (!= (`/Game/BP/FruitsBasketGameInstance.Count` _output_get) 0)
    (bind _cursorlist (`/Game/BP/FruitsBasketGameInstance.CursorList` _output_get))
    (for _array_element _cursorlist
      (switch `string` (`.State_4_DE65D7D94354A3C6D941408BFC6A4A1D` (break `/Game/BP/F_Cursor` _array_element))
        (:`add`
          _)
        (:`update`
          _))
      (set `self.CousorCount` (+ (`self.CousorCount`) 1)))
    (if (== (`self.CousorCount`) 2)
      (bind (_disitance _position _rotation _scale) (`/Game/BP/BPL_Utility.GetBarTransform` _cursorlist))
      (if (>= _disitance (`/Game/BP/FruitsBasketGameInstance.MinimumDistance` (`self.As Separate Fruits Game Instance`)))
        (bind _vector (`/Game/BP/BPL_Utility.FromMeasuredValueToPosition` _position))
        (`self.K2_SetActorLocationAndRotation` (`KismetMathLibrary.MakeVector` (.x _vector) (.y _vector) (- (.z _vector) 10.0)) _rotation)
        (`self.SetActorRelativeScale3D` _scale)
        (else
          (`KismetSystemLibrary.Delay` 0.1 :!label _label)
          (`self.K2_DestroyActor`)))
      (else
        (goto _label)))
    (else
      (goto _label))))

(fn `UserConstructionScript`
  (`PrimitiveComponent.SetUseCCD` (`self.Bar`) true "None"))