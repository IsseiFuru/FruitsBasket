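; BP_Cursor is a cursor actor that represents one entry, selected by SectionID, in the game instance's CursorList.
; Each tick it reads that entry's State: Update moves the actor to the stored measured value converted to a world position, and Remove destroys it after a short delay.
; A TimeLimit check, also run every tick, destroys the cursor when the game instance's Count reaches zero.
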(event `self.ReceiveTick`
  (params (DeltaSeconds :type "Float (single-precision)"))
  (`self.TimeLimit`)
  (bind _asfruits_basket_game_instance (`/Game/BP/BPL_Utility.GetGameInstanceRef`))
  (bind (_state _sessionid _psition) (break `/Game/BP/F_Cursor` (`|GetArrayItem` (`/Game/BP/FruitsBasketGameInstance.CursorList` _asfruits_basket_game_instance) (`self.SectionID`))))
  (switch `string` _state
    (:`update`
      ;[0.01 0.35 1] code : update
      (bind _vector (`/Game/BP/BPL_Utility.FromMeasuredValueToPosition` _psition))
      (`self.K2_SetActorLocation` _vector))
    (:`remove`
      ;[0.01 0.35 1] code : remove
      (`KismetSystemLibrary.Delay` 0.1)
      (`self.K2_DestroyActor`))))

(event `TimeLimit`
  (bind _asfruits_basket_game_instance (`/Game/BP/BPL_Utility.GetGameInstanceRef`))
  (if (== (`/Game/BP/FruitsBasketGameInstance.Count` _asfruits_basket_game_instance) 0)
    (`self.K2_DestroyActor`)))

(fn `UserConstructionScript`)