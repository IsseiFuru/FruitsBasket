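; BP_Apple is a fruit actor that scores when it lands in a matching basket.
; On overlap it casts to BP_AppleBasket and, if FruitsNumber matches, plays a sound and adds points to the GameInstance score.
; After a short delay it destroys itself and decrements the GameInstance FruitsCount.
; The construction script enables CCD on its static mesh for continuous collision detection.
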(event `self.ReceiveActorBeginOverlap`
  (params (OtherActor :type "Actor Object Reference"))
  (bind _asfruits_basket_game_instance (`/Game/BP/BPL_Utility.GetGameInstanceRef`))
  (bind _asbp_apple_basket (cast `/Game/BP/BP_AppleBasket` OtherActor)
    (:`then`
      (if (== (`/Game/BP/BP_AppleBasket.FruitsNumber` _asbp_apple_basket) (`self.FruitsNumber`))
        (`GameplayStatics.PlaySound2D` "/Game/Sound/決定ボタンを押す40.決定ボタンを押す40" 1.0 1.0 0.0 null null)
        (set `/Game/BP/FruitsBasketGameInstance.Score` (+ (`/Game/BP/FruitsBasketGameInstance.Score` _asfruits_basket_game_instance) 1000) _asfruits_basket_game_instance)))
    (:`CastFailed`
      _))
  (`KismetSystemLibrary.Delay` 0.3)
  (`self.K2_DestroyActor`)
  (set `/Game/BP/FruitsBasketGameInstance.FruitsCount` (- (`/Game/BP/FruitsBasketGameInstance.FruitsCount` _asfruits_basket_game_instance) 1) _asfruits_basket_game_instance))

(fn `UserConstructionScript`
  (`PrimitiveComponent.SetUseCCD` (`self.StaticMesh`) true "None"))