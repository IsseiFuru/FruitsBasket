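; Game mode for the Fruits Basket game, running a timed round from ready countdown to the end level.
; On BeginPlay it resets GameInstance state, creates the widgets and spawns the OSC receiver.
; One looping one-second timer drives both countdowns: the ready phase starts music and the fruit spawner, then the round clock raises MaxFruits at set marks.
; At zero it shows the finish widget and opens the End level after a delay.
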(event `self.ReceiveBeginPlay`
  (`self.InitialGameInstance`)
  (`self.Create UI`)
  (`self.Timer`)
  (`self.SpawnOscReceiver`))

(event `InitialGameInstance`
  (bind _asfruits_basket_game_instance (`/Game/BP/BPL_Utility.GetGameInstanceRef`))
  (bind _output_get (set `self.As Fruits Basket Game Instance` _asfruits_basket_game_instance))
  (set `/Game/BP/FruitsBasketGameInstance.CursorList` (`/Game/BP/FruitsBasketGameInstance.DefaultCursorList` _output_get) _output_get)
  (set `/Game/BP/FruitsBasketGameInstance.MinimumDistance` 0.2 _output_get)
  (set `/Game/BP/FruitsBasketGameInstance.FruitsCount` 0 _output_get)
  (set `/Game/BP/FruitsBasketGameInstance.MaxFruits` 1 _output_get)
  (set `/Game/BP/FruitsBasketGameInstance.Readycount` 3 _output_get)
  (set `/Game/BP/FruitsBasketGameInstance.Count` 60 _output_get)
  (set `/Game/BP/FruitsBasketGameInstance.Score` 0 _output_get))

(event `Create UI`
  (bind _returnvalue (`|CreateWidget` "/Game/UI/WBP_ReadyTimer.WBP_ReadyTimer_C"))
  (`UserWidget.AddToViewport` _returnvalue 0)
  (set `self.WBP_ReadyTimer` _returnvalue)
  (bind _returnvalue_2 (`|CreateWidget` "/Game/UI/WBP_Main.WBP_Main_C"))
  (`UserWidget.AddToViewport` _returnvalue_2 0)
  (bind _returnvalue_3 (`|CreateWidget` "/Game/UI/WBP_MainFinish.WBP_MainFinish_C"))
  (set `self.WBP_MainFinish` _returnvalue_3))

(event `Timer`
  (`KismetSystemLibrary.K2_SetTimerDelegate` (delegate `CountDown`) 1.0 true)
  (`GameplayStatics.SpawnSound2D` "/Game/Sound/カウントダウン電子音.カウントダウン電子音" 1.0 1.0 0.0 null))

(event `CountDown`
  (bind _as_fruits_basket_game_instance (`self.As Fruits Basket Game Instance`))
  (bind _count (`/Game/BP/FruitsBasketGameInstance.Count` _as_fruits_basket_game_instance))
  (if (`self.isGameStart`)
    (if (not (<= _count 0))
      (bind _output_get (set `/Game/BP/FruitsBasketGameInstance.Count` (- _count 1) _as_fruits_basket_game_instance))
      (if (or (== _output_get 30) (== _output_get 10))
        (`GameplayStatics.PlaySound2D` "/Game/Sound/決定ボタンを押す24.決定ボタンを押す24" 1.0 1.0 0.0 null null)
        (set `/Game/BP/FruitsBasketGameInstance.MaxFruits` (+ (`/Game/BP/FruitsBasketGameInstance.MaxFruits` _as_fruits_basket_game_instance) 1) _as_fruits_basket_game_instance)
        (elif (== _output_get 0)
          (`self.GameEnd`)
          (elif (<= _output_get 5)
            (`GameplayStatics.PlaySound2D` "/Game/Sound/カウント_Cue.カウント_Cue" 1.0 1.0 0.0 null null)))))
    (else
      (`self.ReadyCountDown`))))

(event `ReadyCountDown`
  (bind _as_fruits_basket_game_instance (`self.As Fruits Basket Game Instance`))
  (bind _readycount (`/Game/BP/FruitsBasketGameInstance.Readycount` _as_fruits_basket_game_instance))
  (if (<= _readycount 0)
    (set `self.isGameStart` true)
    (`self.Play BackMusic`)
    (`self.SpawnFruitsSpawner`)
    (`Widget.RemoveFromParent` (`self.WBP_ReadyTimer`))
    (else
      (set `/Game/BP/FruitsBasketGameInstance.Readycount` (- _readycount 1) _as_fruits_basket_game_instance))))

(event `Play BackMusic`
  (`GameplayStatics.PlaySound2D` "/Game/Sound/fruitsparfait.fruitsparfait" 1.0 1.0 0.0 null null))

(event `GameEnd`
  (`UserWidget.AddToViewport` (`self.WBP_MainFinish`) 0)
  (`GameplayStatics.PlaySound2D` "/Game/Sound/警官のホイッスル2.警官のホイッスル2" 1.0 1.0 0.0 null null)
  (`KismetSystemLibrary.Delay` 2.0)
  (`GameplayStatics.OpenLevelBySoftObjectPtr` "/Game/Map/End.End"))

(event `SpawnOscReceiver`
  (`|SpawnActorFromClass` "/Game/BP/BP_OscReceiver.BP_OscReceiver_C" (`self.NoneStaticMeshTransform`) "Undefined" "OverrideRootScale" null null))

(event `SpawnFruitsSpawner`
  (`|SpawnActorFromClass` "/Game/BP/BP_FruitsSpawner.BP_FruitsSpawner_C" (`self.NoneStaticMeshTransform`) "Undefined" "OverrideRootScale" null null))

(fn `UserConstructionScript`)