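; BP_FruitsSpawner is an actor that spawns falling-fruit candidates (apple, orange or pear) at random horizontal positions at a fixed height.
; Tick reads the GameInstance and, while FruitsCount is below MaxFruits, uses a Delay to throttle spawns to about one per second.
; Each spawn picks a random class with its own transform and increments FruitsCount.
; The spawner destroys itself when the GameInstance's Count reaches zero.
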(event `self.ReceiveTick`
  (params (DeltaSeconds :type "Float (single-precision)"))
  (bind _spawnlocation (`self.SpawnLocation`))
  (bind _asfruits_basket_game_instance (`/Game/BP/BPL_Utility.GetGameInstanceRef`))
  (if (!= (`/Game/BP/FruitsBasketGameInstance.Count` _asfruits_basket_game_instance) 0)
    (if (< (`/Game/BP/FruitsBasketGameInstance.FruitsCount` _asfruits_basket_game_instance) (`/Game/BP/FruitsBasketGameInstance.MaxFruits` _asfruits_basket_game_instance))
      (`KismetSystemLibrary.Delay` 1.0)
      (set `self.SpawnLocation` (`KismetMathLibrary.MakeVector` 0.5 (`KismetMathLibrary.RandomFloatInRange` -500.0 500.0) 450.0))
      (switch `int` (`KismetMathLibrary.RandomInteger` 3)
        (:`0`
          (`|SpawnActorFromClass` "/Game/BP/BP_Apple.BP_Apple_C" (`KismetMathLibrary.MakeTransform` _spawnlocation (struct :`Yaw` 90.0) (2.0 2.0 2.0)) "Undefined" "OverrideRootScale" null null))
        (:`1`
          (`|SpawnActorFromClass` "/Game/BP/BP_Orange.BP_Orange_C" (`KismetMathLibrary.MakeTransform` _spawnlocation (struct :`Roll` 270.0) (600.0 600.0 600.0)) "Undefined" "OverrideRootScale" null null))
        (:`2`
          (`|SpawnActorFromClass` "/Game/BP/BP_Pear.BP_Pear_C" (`KismetMathLibrary.MakeTransform` _spawnlocation (struct) (550.0 550.0 550.0)) "Undefined" "OverrideRootScale" null null)))
      (set `/Game/BP/FruitsBasketGameInstance.FruitsCount` (+ (`/Game/BP/FruitsBasketGameInstance.FruitsCount` _asfruits_basket_game_instance) 1) _asfruits_basket_game_instance))
    (else
      (`self.K2_DestroyActor`))))

(fn `UserConstructionScript`)